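; Elevator actor that handles layout of a Body between bottom and upper border boxes; the file holds no movement logic.
; The construction script only sizes both borders.
; UpdateLocation, not called within this file, snaps Body to the selected border, using mesh bounds for the upper one, and sets the initial direction flag.
; ResetOrigin then shifts the actor origin to the bottom border's height and counter-offsets the three components to keep their world positions.
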(event EventBeginPlay)

(event Collision|EventActorBeginOverlap
  (params (OtherActor :type Actor%20Object%20Reference)))

(event EventTick
  (params (DeltaSeconds :type Float%20%28single-precision%29)))

(fn ConstructionScript
  (CallFunction|SetCollisionSize))

(fn SnaptoBorder
  (params (TargetLocation :type Vector) (Z%20Offset :type Float%20%28double-precision%29))
  (bind _bodylocation (Variables|Default|GetBodyLocation))
  (bind (_x _y) (Math|Vector|BreakVector _bodylocation))
  (Transformation|SetRelativeLocation (Variables|Default|GetBody) (Math|Vector|MakeVector _x _y (- (+ (.Z (Math|Vector|BreakVector TargetLocation)) (.Z (Math|Vector|BreakVector (Variables|Default|GetBoxExtentSize)))) Z%20Offset)) false true))

(fn UpdateLocation
  ;[0.15 0.15 0.15 0.5] Set components' location variables
  (bind _output_get (Variables|Default|SetBottomBorderLocation (Variables|/Script/Engine.SceneComponent|GetRelativeLocation (Variables|Default|GetBottomBorder))))
  (bind _output_get_2 (Variables|Default|SetUpperBorderLocation (Variables|/Script/Engine.SceneComponent|GetRelativeLocation (Variables|Default|GetUpperBorder))))
  (Variables|Default|SetBodyLocation (Variables|/Script/Engine.SceneComponent|GetRelativeLocation (Variables|Default|GetBody)))
  ;[0.15 0.15 0.15 0.5] Snap Body to selected Collision Box and set isAboutToGoDown relevantly
  (if (Variables|Default|GetSnapToUpperBorder)
    (CallFunction|SnaptoBorder _output_get_2 (+ (* (.Z (Math|Vector|BreakVector (.BoxExtent (Collision|GetComponentBounds (Variables|Default|GetBody))))) 2.0) (* (.Z (Math|Vector|BreakVector (Variables|Default|GetBoxExtentSize))) 2.0)))
    (Variables|Default|SetisAboutToGoDown true)
    (else
      (CallFunction|SnaptoBorder _output_get 0.0)
      (Variables|Default|SetisAboutToGoDown false)))
  (CallFunction|ResetOrigin))

(fn SetCollisionSize
  ;[0.15 0.15 0.15 0.5] Set Collision Borders size (Z Axis is a key for Body offset)
  (bind _output_get (Variables|Default|SetBoxExtentSize "250.000000,130.000000,1.000000"))
  (Components|Box|SetBoxExtent (Variables|Default|GetBottomBorder) _output_get false)
  (Components|Box|SetBoxExtent (Variables|Default|GetUpperBorder) _output_get false))

(fn ResetOrigin
  (bind _returnvalue (Transformation|GetActorLocation))
  (bind (_x _y _z) (Math|Vector|BreakVector _returnvalue))
  (bind _output_get (LocalVariables|SetMovedZ (.Z (Math|Vector|BreakVector (Variables|Default|GetBottomBorderLocation)))))
  (Transformation|SetActorLocation (Math|Vector|MakeVector _x _y (+ _z _output_get)) false false)
  (CallFunction|MoveRelative (Variables|Default|GetBody) (LocalVariables|GetMovedZ))
  (CallFunction|MoveRelative (Variables|Default|GetBottomBorder) (LocalVariables|GetMovedZ))
  (CallFunction|MoveRelative (Variables|Default|GetUpperBorder) (LocalVariables|GetMovedZ)))

(fn MoveRelative
  (params (Target%20Component :type Scene%20Component%20Object%20Reference) (Z%20Offset :type Float%20%28double-precision%29))
  (bind _relativelocation (Variables|/Script/Engine.SceneComponent|GetRelativeLocation Target%20Component))
  (bind (_x _y _z) (Math|Vector|BreakVector _relativelocation))
  (Transformation|SetRelativeLocation Target%20Component (Math|Vector|MakeVector _x _y (- _z Z%20Offset)) false false))