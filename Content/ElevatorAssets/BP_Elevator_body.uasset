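; BP_Elevator_body is an elevator body actor with a Body component and two box borders, BottomBorder and UpperBorder.
; The construction script sizes both borders from BoxExtentSize and sets Body's relative height to the BottomBorder's Z plus that extent's Z, keeping its X and Y.
; The event graph holds only disabled placeholder events, so this Blueprint's graphs contain no movement or overlap logic.
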(event EventBeginPlay)

(event Collision|EventActorBeginOverlap
  (params (OtherActor :type Actor%20Object%20Reference)))

(event EventTick
  (params (DeltaSeconds :type Float%20%28single-precision%29)))

(fn ConstructionScript
  (bind _body (Variables|Default|GetBody))
  (bind _boxextentsize (LocalVariables|GetBoxExtentSize))
  (bind _relativelocation (Variables|/Script/Engine.SceneComponent|GetRelativeLocation _body))
  (bind (_x _y) (Math|Vector|BreakVector _relativelocation))
  (Components|Box|SetBoxExtent (Variables|Default|GetBottomBorder) _boxextentsize false)
  (Components|Box|SetBoxExtent (Variables|Default|GetUpperBorder) _boxextentsize false)
  (Transformation|SetRelativeLocation _body (Math|Vector|MakeVector _x _y (+ (.Z (Math|Vector|BreakVector (Variables|/Script/Engine.SceneComponent|GetRelativeLocation (Variables|Default|GetBottomBorder)))) (.Z (Math|Vector|BreakVector (LocalVariables|GetBoxExtentSize))))) false false))